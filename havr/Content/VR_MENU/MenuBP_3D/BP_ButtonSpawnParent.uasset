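; Physical push button for a VR 3D menu that spawns furniture and building pieces, such as chairs, doors and walls.
; While a controller fingertip overlaps it, Tick slides the cube along local Z with clamping, and a timeline snaps it back.
; A full press with the right-hand menu active rumbles and spawns the ItemType/Index actor on the left controller's laser.
; PlaceItem detaches that object and resets placement state.
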(event `self.ReceiveTick`
  (params (DeltaSeconds :type "Float (single-precision)"))
  (bind (_buttonstartlocation_x _buttonstartlocation_y _buttonstartlocation_z) (`KismetMathLibrary.BreakVector` (`self.ButtonStartLocation`)))
  (bind _buttonstartlocation (`self.ButtonStartLocation`))
  (bind _z (.z _buttonstartlocation))
  (bind (_relativelocation_x _relativelocation_y _relativelocation_z) (`KismetMathLibrary.BreakVector` (`SceneComponent.RelativeLocation` (`self.Cube`))))
  (if (not (`self.Controllers Created`))
    (bind _outactors (`GameplayStatics.GetAllActorsOfClass` "/Game/VirtualRealityBP/Blueprints/MotionControllerPawn.MotionControllerPawn_C"))
    (bind _output_get (set `self.motion controller pawn` (`|GetArrayItem` _outactors)))
    (set `self.Left Motion Controller` (`/Game/VirtualRealityBP/Blueprints/MotionControllerPawn.LeftController` _output_get))
    (set `self.Right Motion Controller` (`/Game/VirtualRealityBP/Blueprints/MotionControllerPawn.RightController` _output_get))
    (set `self.Controllers Created` true))
  (`/Engine/EditorBlueprintResources/StandardMacros.Gate` true :!label _label
    (:`Exit`
      (`SceneComponent.K2_SetRelativeLocation` (`self.Cube`) (`KismetMathLibrary.MakeVector` (.x (+ (`KismetMathLibrary.MakeVector` 0.0 0.0 (.z (- (`KismetMathLibrary.InverseTransformLocation` (`self.GetTransform`) (`SceneComponent.K2_GetComponentLocation` (`self.FigerTip`))) (`self.ButtonStartLocation`)))) _buttonstartlocation)) (.y (+ (`KismetMathLibrary.MakeVector` 0.0 0.0 (.z (- (`KismetMathLibrary.InverseTransformLocation` (`self.GetTransform`) (`SceneComponent.K2_GetComponentLocation` (`self.FigerTip`))) (`self.ButtonStartLocation`)))) _buttonstartlocation)) (`KismetMathLibrary.FClamp` (.z (+ (`KismetMathLibrary.MakeVector` 0.0 0.0 (.z (- (`KismetMathLibrary.InverseTransformLocation` (`self.GetTransform`) (`SceneComponent.K2_GetComponentLocation` (`self.FigerTip`))) (`self.ButtonStartLocation`)))) _buttonstartlocation)) (- (`self.PressDistance`) _z) _z)) false false)
      (if (`KismetMathLibrary.NearlyEqual_FloatFloat` _relativelocation_z (- _buttonstartlocation_z (`self.PressDistance`)) 0.1)
        (bind _asbp_motion_controller (cast `/Game/VirtualRealityBP/Blueprints/BP_MotionController` (`ActorComponent.GetOwner` (`self.FigerTip`))))
        (if (`/Game/VirtualRealityBP/Blueprints/BP_MotionController.Is Menu Active` (`self.Right Motion Controller`))
          (`/Game/VirtualRealityBP/Blueprints/BP_MotionController.RumbleController` _asbp_motion_controller 100000000.0)
          (`self.Spawn Item`)
          (`self.ResetButton`))))))

(event `self.Box.OnComponentBeginOverlap`
  (params (OverlappedComponent :type "PrimitiveComponent Object Reference") (OtherActor :type "Actor Object Reference") (OtherComp :type "PrimitiveComponent Object Reference") (OtherBodyIndex :type Integer) (bFromSweep :type Boolean) (SweepResult :type "HitResult Structure (by ref)"))
  (bind _asbp_motion_controller (cast `/Game/VirtualRealityBP/Blueprints/BP_MotionController` OtherActor))
  (`PrimitiveComponent.SetMaterial` (`self.Cube`) 0 "/Game/Models/Appliances/toilet/Ceramic.Ceramic")
  (set `self.IsColliding` true)
  (if (not (`self.DisablePress`))
    (bind _asbp_motion_controller_2 (cast `/Game/VirtualRealityBP/Blueprints/BP_MotionController` OtherActor))
    (bind _fingertip (`/Game/VirtualRealityBP/Blueprints/BP_MotionController.FingerTip` _asbp_motion_controller_2))
    (if (== _fingertip OtherComp)
      (set `self.DisablePress` true)
      (set `self.FigerTip` _fingertip)
      (set `self.ButtonStartLocation` (`SceneComponent.RelativeLocation` (`self.Cube`)))
      (goto _label :!via `Open`))))

(event `ResetButton`
  (`|ExecutionSequence` :!label _label_2
    (:`then_0`
      (goto _label :!via `Close`))
    (:`then_1`
      (bind (_direction _driver) (`Timeline|SnapbackTimeline` :!via `PlayFromStart`)
        (:`Update`
          (`SceneComponent.K2_SetRelativeLocation` (`self.Cube`) (`KismetMathLibrary.MakeVector` (.x (`self.ButtonStartLocation`)) (.y (`self.ButtonStartLocation`)) (`KismetMathLibrary.Lerp` (.z (`SceneComponent.RelativeLocation` (`self.Cube`))) (.z (`self.ButtonStartLocation`)) _driver)) false false))
        (:`Finished`
          (set `self.DisablePress` false))))))

(event `self.Box.OnComponentEndOverlap`
  (params (OverlappedComponent :type "PrimitiveComponent Object Reference") (OtherActor :type "Actor Object Reference") (OtherComp :type "PrimitiveComponent Object Reference") (OtherBodyIndex :type Integer))
  (bind _asbp_motion_controller (cast `/Game/VirtualRealityBP/Blueprints/BP_MotionController` OtherActor)
    (:`then`
      (`PrimitiveComponent.SetMaterial` (`self.Cube`) 0 "/Game/Geometry/Meshes/CubeMaterial.CubeMaterial")
      (set `self.IsColliding` false))
    (:`CastFailed`
      _))
  (bind _asbp_motion_controller_2 (cast `/Game/VirtualRealityBP/Blueprints/BP_MotionController` OtherActor))
  (if (== (`/Game/VirtualRealityBP/Blueprints/BP_MotionController.FingerTip` _asbp_motion_controller_2) OtherComp)
    (goto _label_2)))

(fn `Place Item`
  (bind _motion_controller_pawn (`self.motion controller pawn`))
  (bind _left_motion_controller (`self.Left Motion Controller`))
  (`SceneComponent.K2_DetachFromComponent` (`Actor.RootComponent` (`self.Spawned Object`)) "KeepWorld" "KeepWorld" "KeepWorld" true)
  (set `/Game/VirtualRealityBP/Blueprints/BP_MotionController.ObjectAttached` false _left_motion_controller)
  (`KismetArrayLibrary.Array_Clear` (`/Game/VirtualRealityBP/Blueprints/BP_MotionController.Actors to Ignore` _left_motion_controller))
  (set `/Game/VirtualRealityBP/Blueprints/BP_MotionController.Laser Scale` (0.01 0.01 0.01) _left_motion_controller)
  (set `/Game/VirtualRealityBP/Blueprints/MotionControllerPawn.Scale Amount` 0.01 _motion_controller_pawn)
  (set `/Game/VirtualRealityBP/Blueprints/MotionControllerPawn.rotation amount` 0.0 _motion_controller_pawn))

(fn `PushButton`)

(fn `Spawn Item`
  (bind _left_motion_controller (`self.Left Motion Controller`))
  (bind _spawned_object (`self.Spawned Object`))
  (if (not (`/Game/VirtualRealityBP/Blueprints/BP_MotionController.ObjectAttached` (`self.Left Motion Controller`)))
    (switch `string` (`self.ItemType`)
      (:`Chair`
        (bind _asactor (castclass `Actor` (`|GetArrayItem` (`self.Chairs`) (`self.Index`))))
        (bind _returnvalue (`|SpawnActorFromClass` _asactor (`KismetMathLibrary.MakeTransform` (`/Game/VirtualRealityBP/Blueprints/BP_MotionController.LaserHit` (`self.Left Motion Controller`))) "AdjustIfPossibleButAlwaysSpawn" "OverrideRootScale" null null))
        (set `self.Spawned Object` _returnvalue)
        (`self.K2_AttachToComponent` _returnvalue (`/Game/VirtualRealityBP/Blueprints/BP_MotionController. Laser Collision Point` (`self.Left Motion Controller`)) "None" "KeepWorld" "KeepWorld" "KeepWorld" true))
      (:`Table`
        (bind _asactor_2 (castclass `Actor` (`|GetArrayItem` (`self.Tables`) (`self.Index`))))
        (bind _returnvalue_2 (`|SpawnActorFromClass` _asactor_2 (`KismetMathLibrary.MakeTransform` (`/Game/VirtualRealityBP/Blueprints/BP_MotionController.LaserHit` (`self.Left Motion Controller`))) "AdjustIfPossibleButAlwaysSpawn" "OverrideRootScale" null null))
        (set `self.Spawned Object` _returnvalue_2)
        (`self.K2_AttachToComponent` _returnvalue_2 (`/Game/VirtualRealityBP/Blueprints/BP_MotionController. Laser Collision Point` (`self.Left Motion Controller`)) "None" "KeepRelative" "KeepWorld" "KeepWorld" true))
      (:`Couch`
        (bind _asactor_3 (castclass `Actor` (`|GetArrayItem` (`self.Couches`) (`self.Index`))))
        (bind _returnvalue_3 (`|SpawnActorFromClass` _asactor_3 (`KismetMathLibrary.MakeTransform` (`/Game/VirtualRealityBP/Blueprints/BP_MotionController.LaserHit` (`self.Left Motion Controller`))) "AdjustIfPossibleButAlwaysSpawn" "OverrideRootScale" null null))
        (set `self.Spawned Object` _returnvalue_3)
        (`self.K2_AttachToComponent` _returnvalue_3 (`/Game/VirtualRealityBP/Blueprints/BP_MotionController. Laser Collision Point` (`self.Left Motion Controller`)) "None" "KeepWorld" "KeepWorld" "KeepWorld" true))
      (:`Door`
        (bind _asactor_4 (castclass `Actor` (`|GetArrayItem` (`self.Doors`) (`self.Index`))))
        (bind _returnvalue_4 (`|SpawnActorFromClass` _asactor_4 (`KismetMathLibrary.MakeTransform` (`/Game/VirtualRealityBP/Blueprints/BP_MotionController.LaserHit` (`self.Left Motion Controller`))) "AdjustIfPossibleButAlwaysSpawn" "OverrideRootScale" null null))
        (set `self.Spawned Object` _returnvalue_4)
        (`self.K2_AttachToComponent` _returnvalue_4 (`/Game/VirtualRealityBP/Blueprints/BP_MotionController. Laser Collision Point` (`self.Left Motion Controller`)) "None" "KeepWorld" "KeepWorld" "KeepWorld" true))
      (:`Appliance`
        (bind _asactor_5 (castclass `Actor` (`|GetArrayItem` (`self.Appliances`) (`self.Index`))))
        (bind _returnvalue_5 (`|SpawnActorFromClass` _asactor_5 (`KismetMathLibrary.MakeTransform` (`/Game/VirtualRealityBP/Blueprints/BP_MotionController.LaserHit` (`self.Left Motion Controller`))) "AdjustIfPossibleButAlwaysSpawn" "OverrideRootScale" null null))
        (set `self.Spawned Object` _returnvalue_5)
        (`self.K2_AttachToComponent` _returnvalue_5 (`/Game/VirtualRealityBP/Blueprints/BP_MotionController. Laser Collision Point` (`self.Left Motion Controller`)) "None" "KeepWorld" "KeepWorld" "KeepWorld" true))
      (:`Bed`
        (bind _asactor_6 (castclass `Actor` (`|GetArrayItem` (`self.Beds`) (`self.Index`))))
        (bind _returnvalue_6 (`|SpawnActorFromClass` _asactor_6 (`KismetMathLibrary.MakeTransform` (`/Game/VirtualRealityBP/Blueprints/BP_MotionController.LaserHit` (`self.Left Motion Controller`))) "AdjustIfPossibleButAlwaysSpawn" "OverrideRootScale" null null))
        (set `self.Spawned Object` _returnvalue_6)
        (`self.K2_AttachToComponent` _returnvalue_6 (`/Game/VirtualRealityBP/Blueprints/BP_MotionController. Laser Collision Point` (`self.Left Motion Controller`)) "None" "KeepWorld" "KeepWorld" "KeepWorld" true))
      (:`Other`
        (bind _asactor_7 (castclass `Actor` (`|GetArrayItem` (`self.Other`) (`self.Index`))))
        (bind _returnvalue_7 (`|SpawnActorFromClass` _asactor_7 (`KismetMathLibrary.MakeTransform` (`/Game/VirtualRealityBP/Blueprints/BP_MotionController.LaserHit` (`self.Left Motion Controller`))) "AdjustIfPossibleButAlwaysSpawn" "OverrideRootScale" null null))
        (set `self.Spawned Object` _returnvalue_7)
        (`self.K2_AttachToComponent` _returnvalue_7 (`/Game/VirtualRealityBP/Blueprints/BP_MotionController. Laser Collision Point` (`self.Left Motion Controller`)) "None" "KeepWorld" "KeepWorld" "KeepWorld" true))
      (:`Wall`
        (bind _asactor_8 (castclass `Actor` (`|GetArrayItem` (`self.Walls`) (`self.Index`))))
        (bind _returnvalue_8 (`|SpawnActorFromClass` _asactor_8 (`KismetMathLibrary.MakeTransform` (`/Game/VirtualRealityBP/Blueprints/BP_MotionController.LaserHit` (`self.Left Motion Controller`))) "AdjustIfPossibleButAlwaysSpawn" "OverrideRootScale" null null))
        (set `self.Spawned Object` _returnvalue_8)
        (`self.K2_AttachToComponent` _returnvalue_8 (`/Game/VirtualRealityBP/Blueprints/BP_MotionController. Laser Collision Point` (`self.Left Motion Controller`)) "None" "KeepWorld" "KeepWorld" "KeepWorld" true)))
    (set `/Game/VirtualRealityBP/Blueprints/BP_MotionController.ObjectAttached` true _left_motion_controller)
    (set `/Game/VirtualRealityBP/Blueprints/BP_MotionController.Spawned Object Type` (`self.ItemType`) _left_motion_controller)
    (set `/Game/VirtualRealityBP/Blueprints/BP_MotionController.Spawned object index` (`self.Index`) _left_motion_controller)
    (`KismetArrayLibrary.Array_Add` (`/Game/VirtualRealityBP/Blueprints/BP_MotionController.Actors to Ignore` _left_motion_controller) _spawned_object)
    (set `/Game/VirtualRealityBP/Blueprints/BP_MotionController.SpawnedObject` _spawned_object _left_motion_controller)))

(fn `UserConstructionScript`
  (`TextRenderComponent.K2_SetText` (`self.Wall_txt`) (`self.ButtonText`)))